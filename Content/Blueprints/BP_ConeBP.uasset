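; BP_ConeBP is an actor that bobs vertically between its starting height and a configurable distance above it.
; BeginPlay records the start Z as the lower bound and adds Max to set the upper bound.
; Each Tick moves the height by Speed times delta time, flips direction past either bound, and sets the location without sweep, keeping X and Y.
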(event `self.ReceiveBeginPlay`
  (bind (_returnvalue_x _returnvalue_y _returnvalue_z) (`KismetMathLibrary.BreakVector` (`self.K2_GetActorLocation`)))
  (set `self.bIsUp` true)
  (set `self.CurrentHeight` _returnvalue_z)
  (set `self.MinHeight` _returnvalue_z)
  (set `self.MaxHeight` (+ _returnvalue_z (`self.Max`))))

(event `self.ReceiveTick`
  (params (DeltaSeconds :type "Float (single-precision)"))
  (bind (_returnvalue_x _returnvalue_y) (`KismetMathLibrary.BreakVector` (`self.K2_GetActorLocation`)))
  (bind _returnvalue (* DeltaSeconds (`self.Speed`)))
  (if (`self.bIsUp`)
    (set `self.CurrentHeight` (+ (`self.CurrentHeight`) _returnvalue))
    (else
      (set `self.CurrentHeight` (- (`self.CurrentHeight`) _returnvalue))))
  (`self.K2_SetActorLocation` (`KismetMathLibrary.MakeVector` _returnvalue_x _returnvalue_y (`self.CurrentHeight`)))
  (if (> (`self.CurrentHeight`) (`self.MaxHeight`))
    (set `self.bIsUp` false))
  (if (< (`self.CurrentHeight`) (`self.MinHeight`))
    (set `self.bIsUp` true)))

(fn `UserConstructionScript`)